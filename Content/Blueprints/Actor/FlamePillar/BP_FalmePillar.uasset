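; Flame pillar actor whose fire light can flicker and jitter.
; The construction script gives FireLight a dynamic MI_FireLight light function with a random "Randomness Shift", so each instance varies.
; If MoveLightSource is set, BeginPlay starts a looping timer that nudges the light toward random points in a small box above the actor.
; Each timer call makes one VInterpTo step using frame delta time, rather than interpolating every tick.
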(event `self.ReceiveBeginPlay`
  (if (`self.MoveLightSource`)
    (`KismetSystemLibrary.K2_SetTimerDelegate` (delegate `MoveLight`) 0.3 true)))

(event `MoveLight`
  (bind _firelight (`self.FireLight`))
  (bind _output_get (set `self.PreviousLocation` (`SceneComponent.K2_GetComponentLocation` _firelight)))
  (`SceneComponent.K2_SetWorldLocation` _firelight (`KismetMathLibrary.VInterpTo` _output_get (`KismetMathLibrary.RandomPointInBoundingBox` (+ (`self.K2_GetActorLocation`) (0.0 0.0 280.0)) (`KismetMathLibrary.MakeVector` 2.0 2.0 (`KismetMathLibrary.RandomFloatInRange` 0.0 10.0))) (`GameplayStatics.GetWorldDeltaSeconds`) 20.0) false false))

(fn `UserConstructionScript`
  (bind _returnvalue (`KismetMaterialLibrary.CreateDynamicMaterialInstance` "/Game/Blueprints/Actor/FlamePillar/MI_FireLight.MI_FireLight"))
  (`LightComponent.SetLightFunctionMaterial` (`self.FireLight`) _returnvalue)
  (`MaterialInstanceDynamic.SetScalarParameterValue` _returnvalue "Randomness Shift" (`KismetMathLibrary.RandomFloatInRange` -0.5 0.5)))