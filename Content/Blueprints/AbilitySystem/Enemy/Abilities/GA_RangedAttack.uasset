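; Enemy ranged attack gameplay ability that fires a projectile at the avatar's combat target.
; On activation it turns the avatar toward the target through CombatInterface, then plays a random tagged attack montage.
; A gameplay event matching the montage's tag triggers the spawn from that montage's socket, using the target's location at that moment and an optional pitch override.
; The ability ends when the montage completes, is interrupted or is cancelled.
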(event `self.K2_ActivateAbility`
  (`|ExecutionSequence`
    (:`then_0`
      (bind _returnvalue (message `EnemyInterface.GetCombatTarget` (`self.GetAvatarActorFromActorInfo`)))
      (bind _ascombat_interface (cast `CombatInterface` (`self.GetAvatarActorFromActorInfo`)))
      (`CombatInterface.UpdateFacingTarget` _ascombat_interface (`Actor.K2_GetActorLocation` _returnvalue)))
    (:`then_1`
      (bind _returnvalue_2 (message `CombatInterface.GetAttackMontages` (`self.GetAvatarActorFromActorInfo`)))
      (bind _output_get (set `self.TaggedMontage` (`self.GetRandomTaggedMontageFromArray` _returnvalue_2)))
      (bind (_montage _montagetag _sockettag) (break `TaggedMontage` _output_get))
      (`AbilityTask_PlayMontageAndWait.CreatePlayMontageAndWaitProxy` "None" _montage
        (:`then`
          (`AbilityTask_WaitGameplayEvent.WaitGameplayEvent` _montagetag null true
            (:`EventReceived`
              (bind _returnvalue_3 (message `EnemyInterface.GetCombatTarget` (`self.GetAvatarActorFromActorInfo`)))
              (`self.SpawnProjectile` (`Actor.K2_GetActorLocation` _returnvalue_3) _sockettag (`self.ShoudOverridePitch`) (`self.PitchOverride`)))))
        (:`OnCompleted`
          (`self.K2_EndAbility` :!label _label))
        (:`OnInterrupted`
          (goto _label))
        (:`OnCancelled`
          (goto _label))))))

(event `self.K2_OnEndAbility`
  (params (bWasCancelled :type Boolean))
  (`self.K2_EndAbility`))