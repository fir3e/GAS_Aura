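; Enemy melee attack ability that turns the avatar toward its combat target and plays a random tagged attack montage.
; When the montage's gameplay event arrives, it runs a small radius check for live players at the montage's combat socket and damages non-friendly ones.
; A hit fires a melee impact gameplay cue carrying the montage tag and socket location.
; The ability ends after that check or when the montage completes or is interrupted.
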(event `self.K2_ActivateAbility`
  (bind _returnvalue (`self.GetAvatarActorFromActorInfo`))
  (bind _returnvalue_2 (`self.GetAvatarActorFromActorInfo`))
  (bind _returnvalue_3 (`self.GetAvatarActorFromActorInfo`))
  (set `self.HasHitTarget` false)
  (`|ExecutionSequence`
    (:`then_0`
      (bind _returnvalue_4 (message `EnemyInterface.GetCombatTarget` _returnvalue_2))
      (set `self.CombatTarget` _returnvalue_4)
      (bind _ascombat_interface (cast `CombatInterface` _returnvalue_2))
      (bind _output_get (set `self.CombatInterface` _ascombat_interface))
      (`CombatInterface.UpdateFacingTarget` _output_get (`Actor.K2_GetActorLocation` (`self.CombatTarget`))))
    (:`then_1`
      (bind _returnvalue_5 (message `CombatInterface.GetAttackMontages` (`self.GetAvatarActorFromActorInfo`)))
      (bind _output_get_2 (set `self.TaggedMontage` (`self.GetRandomTaggedMontageFromArray` _returnvalue_5)))
      (bind (_montage _montagetag _sockettag) (break `TaggedMontage` _output_get_2))
      (`AbilityTask_PlayMontageAndWait.CreatePlayMontageAndWaitProxy` "None" _montage 1.0 "None" false
        (:`then`
          (`AbilityTask_WaitGameplayEvent.WaitGameplayEvent` _montagetag null
            (:`EventReceived`
              (bind _returnvalue_6 (message `CombatInterface.GetCombatSocketLocation` _returnvalue_3 _sockettag))
              (bind _output_get_3 (set `self.CombatSocketLocation` _returnvalue_6))
              (bind _outoverlappingactors (`AuraAbilitySystemLibrary.GetLivePlayersWithinRadius` _returnvalue_3 (`|MakeArray` _returnvalue_3) 45.0 _output_get_3))
              (for _array_element _outoverlappingactors
                (if (`AuraAbilitySystemLibrary.IsNotFriend` (`self.GetAvatarActorFromActorInfo`) _array_element)
                  (`self.CauseDamage` _array_element)
                  (set `self.HasHitTarget` true)))
              (if (`self.HasHitTarget`)
                (bind _returnvalue_7 (message `EnemyInterface.GetCombatTarget` _returnvalue))
                (`self.K2_ExecuteGameplayCueWithParams` (struct :`TagName` "GameplayCue.MeleeImpact") (`AbilitySystemBlueprintLibrary.MakeGameplayCueParameters` 0.0 0.0 (struct) (struct) (struct) (`BlueprintGameplayTagLibrary.MakeGameplayTagContainerFromTag` (`.MontageTag` (break `TaggedMontage` (`self.TaggedMontage`)))) (struct) (`self.CombatSocketLocation`) (0.0 0.0 0.0) null _returnvalue _returnvalue_7)))
              (`self.K2_EndAbility`))))
        (:`OnCompleted`
          (`self.K2_EndAbility` :!label _label))
        (:`OnInterrupted`
          (goto _label))
        (:`OnCancelled`
          (goto _label))))))

(event `self.K2_OnEndAbility`
  (params (bWasCancelled :type Boolean))
  (`self.K2_EndAbility`))